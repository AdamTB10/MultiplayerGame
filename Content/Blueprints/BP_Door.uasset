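; BP_Door is a door that swings open and closed, apparently networked, judging by its SERVER and MULTI event names.
; Server events pass open and close requests to the multicast events only while PlayTimeline is true, blocking requests mid-swing.
; The multicast events play separate Open and Close timelines that drive the Door's yaw through a 90-degree range.
; When a timeline finishes, it updates IsOpen and re-enables requests; the file contains no caller.
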(event Custom|MULTI_OpenDoor
  (Variables|Default|SetplayTimeline false)
  (bind _rotation (Timeline|Open PlayFromStart)
    (:Update
      (Transformation|SetRelativeRotation (Variables|Default|GetDoor) (Math|Rotator|MakeRotator 0.0 0.0 (* _rotation 9e+01)) false false))
    (:Finished
      (Variables|Default|SetisOpen true)
      (Variables|Default|SetplayTimeline true))))

(event Custom|SERVER_OpenDoor
  (if (Variables|Default|GetplayTimeline)
    (CallFunction|MULTIOpenDoor)))

(event Custom|SERVER_CloseDoor
  (if (Variables|Default|GetplayTimeline)
    (CallFunction|MULTICloseDoor)))

(event Custom|MULTI_CloseDoor
  (Variables|Default|SetplayTimeline false)
  (bind _rotation (Timeline|Close PlayFromStart)
    (:Update
      (Transformation|SetRelativeRotation (Variables|Default|GetDoor) (Math|Rotator|MakeRotator 0.0 0.0 (* _rotation 9e+01)) false false))
    (:Finished
      (Variables|Default|SetisOpen false)
      (Variables|Default|SetplayTimeline true))))

(fn ConstructionScript)