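; Multiplayer player state that tracks a player's Points and keeps score displays in sync.
; Server events add one point or remove two, clamped at zero, with point loss also playing a hit sound for the owner.
; Owner events refresh the score via BP_PlayerController, and multicast events update the pawn's overhead UI through BP_Player.
; The Points OnRep triggers the same two display updates.
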(event Custom|SERVER_AddPoints
  (Math|Integer|IncrementInt (Variables|Default|Getpoints)
    (:%20%20
      (CallFunction|OWNERHUDUpdateScore)
      (CallFunction|MULTIOverHeadUIUpdateScore))))

(event Custom|OWNER_HUDUpdateScore
  (bind _asbp_player_controller (Utilities|Casting|CastToBP_PlayerController (Game|GetPlayerController)))
  (Default|UpdateScore _asbp_player_controller))

(event Custom|MULTI_OverHeadUIUpdateScore
  (bind _asbp_player (Utilities|Casting|CastToBP_Player (PlayerState|GetPawn)))
  (Default|UpdateScore _asbp_player))

(event Custom|SERVER_LoosePoints
  (if (>= (- (Variables|Default|Getpoints) 2) 0)
    (Variables|Default|Setpoints (- (Variables|Default|Getpoints) 2))
    (else
      (Variables|Default|Setpoints 0)))
  (CallFunction|OWNERHUDUpdateScore)
  (CallFunction|MULTIOverHeadUIUpdateScore)
  (CallFunction|OWNERPlayHitSound))

(event Custom|OWNER_PlayHitSound
  (Audio|PlaySound2D "/Game/Audio/SW_Hit.SW_Hit" 1.0 1.0 0.0 0 0))

(fn ConstructionScript)

(fn OnRepPoints
  (CallFunction|OWNERHUDUpdateScore)
  (CallFunction|MULTIOverHeadUIUpdateScore))