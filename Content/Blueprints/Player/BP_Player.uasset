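; Multiplayer player Blueprint that moves, turns on yaw, fires attacks and drops coins.
; Shooting is gated by the PlayerState's attack flag, which is disabled after each shot, while a server event spawns a regular or homing attack by attack type.
; Dropping a coin spawns it behind the player and deducts a point, if any remain.
; An overhead widget receives the PlayerState name and score through MULTI events after a startup delay.
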(event Custom|MULTI_updateName
  (params (name :type Text))
  (Variables|/Script/UMG.TextBlock|SetText (Variables|/Game/UI/WBP_OverHeadUI.WBP_OverHeadUI_C|GetplayerNameUI (Variables|Default|GetoverHeadUI)) name))

(event Custom|MULTI_updateScore
  (bind _asbp_player_state (Utilities|Casting|CastToBP_PlayerState (Variables|GetPlayerState)))
  (Variables|/Script/UMG.TextBlock|SetText (Variables|/Game/UI/WBP_OverHeadUI.WBP_OverHeadUI_C|GetplayerScoreUI (Variables|Default|GetoverHeadUI)) (Utilities|Text|ToText(Integer) (Variables|/Game/Blueprints/Player/BP_PlayerState.BP_PlayerState_C|Getpoints _asbp_player_state))))

(event Custom|SERVER_dropCoin
  (bind _asbp_player_state (Utilities|Casting|CastToBP_PlayerState (Variables|GetPlayerState)))
  (if (> (Variables|/Game/Blueprints/Player/BP_PlayerState.BP_PlayerState_C|Getpoints _asbp_player_state) 0)
    (Game|SpawnActorfromClass "/Game/Blueprints/Interactables/BP_Coin.BP_Coin_C" (Math|Transform|MakeTransform (+ (* (Transformation|GetActorForwardVector) -1e+02) (Transformation|GetActorLocation) "0.000000,0.000000,-50.000000") "0, 0, 0" "1.000000,1.000000,1.000000") "Undefined" "MultiplyWithRoot" 0 0)
    (Default|SERVERLoosePoints _asbp_player_state 1)))

(event Custom|SERVER_Shoot
  (bind _asbp_player_state (Utilities|Casting|CastToBP_PlayerState (Variables|GetPlayerState)))
  (switch Utilities|FlowControl|Switch|SwitchonE_AttackType (Variables|/Game/Blueprints/Player/BP_PlayerState.BP_PlayerState_C|GetattackType _asbp_player_state)
    (:NewEnumerator0
      (Game|SpawnActorfromClass "/Game/Blueprints/Interactables/BP_Attack.BP_Attack_C" (Transformation|GetWorldTransform (Variables|Default|GetBulletSpawn)) "Undefined" "MultiplyWithRoot" 0 0))
    (:NewEnumerator1
      (Game|SpawnActorfromClass "/Game/Blueprints/Interactables/BP_HomingAttack.BP_HomingAttack_C" (Transformation|GetWorldTransform (Variables|Default|GetBulletSpawn)) "Undefined" "MultiplyWithRoot" 0 0))))

(event Input|EnhancedActionEvents|EnhancedInputActionIA_Move
  (params (ActionValue :type Vector%202D%20Structure) (ElapsedSeconds :type Float%20%28double-precision%29) (TriggeredSeconds :type Float%20%28double-precision%29) (InputAction :type Input%20Action%20Object%20Reference :default "/Game/Input/IA_Move.IA_Move"))
  (Pawn|Input|AddMovementInput (Math|Vector|GetForwardVector (Pawn|GetControlRotation :!class /Script/Engine.Pawn)) (.x ActionValue) false)
  (Pawn|Input|AddMovementInput (Math|Vector|GetRightVector (Pawn|GetControlRotation :!class /Script/Engine.Pawn)) (.y ActionValue) false))

(event Input|EnhancedActionEvents|EnhancedInputActionIA_Look
  (params (ActionValue :type Vector%202D%20Structure) (ElapsedSeconds :type Float%20%28double-precision%29) (TriggeredSeconds :type Float%20%28double-precision%29) (InputAction :type Input%20Action%20Object%20Reference :default "/Game/Input/IA_Look.IA_Look"))
  (Pawn|Input|AddControllerYawInput (.x ActionValue)))

(event Input|EnhancedActionEvents|EnhancedInputActionIA_Shoot
  (params (ActionValue :type Boolean) (ElapsedSeconds :type Float%20%28double-precision%29) (TriggeredSeconds :type Float%20%28double-precision%29) (InputAction :type Input%20Action%20Object%20Reference :default "/Game/Input/IA_Shoot.IA_Shoot"))
  (:Started
    (bind _asbp_player_state (Utilities|Casting|CastToBP_PlayerState (Variables|GetPlayerState)))
    (if (Variables|/Game/Blueprints/Player/BP_PlayerState.BP_PlayerState_C|GetcanPlayerAttack _asbp_player_state)
      (CallFunction|SERVERShoot)
      (bind _asbp_player_state_2 (Utilities|Casting|CastToBP_PlayerState (Variables|GetPlayerState)))
      (Default|SERVERDisableCanPlayerAttack _asbp_player_state_2))))

(event Input|EnhancedActionEvents|EnhancedInputActionIA_DropCoin
  (params (ActionValue :type Boolean) (ElapsedSeconds :type Float%20%28double-precision%29) (TriggeredSeconds :type Float%20%28double-precision%29) (InputAction :type Input%20Action%20Object%20Reference :default "/Game/Input/IA_DropCoin.IA_DropCoin"))
  (:Started
    (CallFunction|SERVERDropCoin)))

(event EventBeginPlay
  (Variables|Default|SetcanShoot true)
  (bind _aswbp_over_head_ui (Utilities|Casting|CastToWBP_OverHeadUI (UserInterface|GetWidget (Variables|Default|GetoverHeadWidget))))
  (Variables|Default|SetoverHeadUI _aswbp_over_head_ui)
  (Utilities|FlowControl|Delay 2.5)
  (CallFunction|MULTIUpdateScore)
  (bind _asbp_player_state (Utilities|Casting|CastToBP_PlayerState (Variables|GetPlayerState)))
  (CallFunction|MULTIUpdateName (Variables|/Game/Blueprints/Player/BP_PlayerState.BP_PlayerState_C|Getname _asbp_player_state)))

(fn ConstructionScript)