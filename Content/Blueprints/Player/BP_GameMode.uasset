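; Game mode that runs timed pickup waves and flags the match over in BP_GameState when waves run out.
; Each wave scatters mostly coins, plus rare attack pickups, at random points within every BP_SpawnZones actor's bounds, and centre coins in BP_CentreArea.
; A timer triggers ClearItems, which destroys coins and regular attack pickups, respawns, then increments the wave and sends it to the game state.
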(event Custom|SpawnPickups
  (bind _centrearea (Variables|Default|GetcentreArea))
  (bind (_origin _boxextent) (Collision|GetActorBounds _centrearea false false))
  (bind _returnvalue (Math|Random|RandomPointinBoundingBox (Math|Vector|MakeVector (.x _origin) (.y _origin) (.z _origin)) _boxextent))
  (if (< (Variables|Default|GetcurrentWave) (Variables|Default|GetmaxWaves))
    (for _array_element (Variables|Default|GetListOfSpawnZones)
      (for _index (range 0 (Variables|Default|GetspawnAmount))
        (Variables|Default|SetitemSpawnHeight (- (.z (.Origin (Collision|GetActorBounds _array_element false false))) 5e+01))
        (if (>= (Math|Random|RandomFloat) 0.95)
          (if (< (Math|Random|RandomFloat) 0.7)
            (Game|SpawnActorfromClass "/Game/Blueprints/Interactables/BP_RegularAttackPickUp.BP_RegularAttackPickUp_C" (Math|Transform|MakeTransform (Math|Vector|MakeVector (.x (Math|Random|RandomPointinBoundingBox (Math|Vector|MakeVector (.x (.Origin (Collision|GetActorBounds _array_element false false))) (.y (.Origin (Collision|GetActorBounds _array_element false false))) (.z (.Origin (Collision|GetActorBounds _array_element false false)))) (.BoxExtent (Collision|GetActorBounds _array_element false false)))) (.y (Math|Random|RandomPointinBoundingBox (Math|Vector|MakeVector (.x (.Origin (Collision|GetActorBounds _array_element false false))) (.y (.Origin (Collision|GetActorBounds _array_element false false))) (.z (.Origin (Collision|GetActorBounds _array_element false false)))) (.BoxExtent (Collision|GetActorBounds _array_element false false)))) (Variables|Default|GetitemSpawnHeight)) "0, 0, 0" "1.000000,1.000000,1.000000") "Undefined" "MultiplyWithRoot" 0 0)
            (else
              (Game|SpawnActorfromClass "/Game/Blueprints/Interactables/BP_HomingAttackPickup.BP_HomingAttackPickup_C" (Math|Transform|MakeTransform (Math|Vector|MakeVector (.x (Math|Random|RandomPointinBoundingBox (Math|Vector|MakeVector (.x (.Origin (Collision|GetActorBounds _array_element false false))) (.y (.Origin (Collision|GetActorBounds _array_element false false))) (.z (.Origin (Collision|GetActorBounds _array_element false false)))) (.BoxExtent (Collision|GetActorBounds _array_element false false)))) (.y (Math|Random|RandomPointinBoundingBox (Math|Vector|MakeVector (.x (.Origin (Collision|GetActorBounds _array_element false false))) (.y (.Origin (Collision|GetActorBounds _array_element false false))) (.z (.Origin (Collision|GetActorBounds _array_element false false)))) (.BoxExtent (Collision|GetActorBounds _array_element false false)))) (Variables|Default|GetitemSpawnHeight)) "0, 0, 0" "1.000000,1.000000,1.000000") "Undefined" "MultiplyWithRoot" 0 0)))
          (else
            (Game|SpawnActorfromClass "/Game/Blueprints/Interactables/BP_Coin.BP_Coin_C" (Math|Transform|MakeTransform (Math|Vector|MakeVector (.x (Math|Random|RandomPointinBoundingBox (Math|Vector|MakeVector (.x (.Origin (Collision|GetActorBounds _array_element false false))) (.y (.Origin (Collision|GetActorBounds _array_element false false))) (.z (.Origin (Collision|GetActorBounds _array_element false false)))) (.BoxExtent (Collision|GetActorBounds _array_element false false)))) (.y (Math|Random|RandomPointinBoundingBox (Math|Vector|MakeVector (.x (.Origin (Collision|GetActorBounds _array_element false false))) (.y (.Origin (Collision|GetActorBounds _array_element false false))) (.z (.Origin (Collision|GetActorBounds _array_element false false)))) (.BoxExtent (Collision|GetActorBounds _array_element false false)))) (Variables|Default|GetitemSpawnHeight)) "0, 0, 0" "1.000000,1.000000,1.000000") "Undefined" "MultiplyWithRoot" 0 0)))))
    (for _index_2 (range 0 (Variables|Default|GetspawnAmount))
      (Variables|Default|SetitemSpawnHeight (- (.z _origin) 5e+01))
      (Game|SpawnActorfromClass "/Game/Blueprints/Interactables/BP_CentreArea_Coin.BP_CentreArea_Coin_C" (Math|Transform|MakeTransform (Math|Vector|MakeVector (.x _returnvalue) (.y _returnvalue) (Variables|Default|GetitemSpawnHeight)) "0, 0, 0" "1.000000,1.000000,1.000000") "Undefined" "MultiplyWithRoot" 0 0))
    (Utilities|Time|SetTimerbyEvent (delegate Custom|ClearItems) 6e+01)
    (else
      (CallFunction|EndGame))))

(event Custom|ClearItems
  (bind _outactors (Actor|GetAllActorsOfClass "/Game/Blueprints/Interactables/BP_Coin.BP_Coin_C"))
  (for _array_element _outactors
    (Actor|DestroyActor _array_element))
  (bind _outactors_2 (Actor|GetAllActorsOfClass "/Game/Blueprints/Interactables/BP_RegularAttackPickUp.BP_RegularAttackPickUp_C"))
  (for _array_element_2 _outactors_2
    (Actor|DestroyActor _array_element_2))
  (CallFunction|SpawnPickups)
  (Math|Integer|IncrementInt (Variables|Default|GetcurrentWave)
    (:%20%20
      (bind _asbp_game_state (Utilities|Casting|CastToBP_GameState (Game|GetGameState)))
      (Default|SERVERSetWaveCount _asbp_game_state (Variables|Default|GetcurrentWave) (Variables|Default|GetmaxWaves)))))

(event Custom|EndGame
  (bind _asbp_game_state (Utilities|Casting|CastToBP_GameState (Game|GetGameState)))
  (Variables|/Game/Blueprints/Player/BP_GameState.BP_GameState_C|SetIsMatchOver _asbp_game_state true))

(event EventBeginPlay
  (bind _outactors (Actor|GetAllActorsOfClass "/Game/Blueprints/Level/BP_SpawnZones.BP_SpawnZones_C"))
  (Variables|Default|SetListOfSpawnZones _outactors)
  (bind _returnvalue (Actor|GetActorOfClass "/Game/Blueprints/Level/BP_CentreArea.BP_CentreArea_C"))
  (Variables|Default|SetcentreArea _returnvalue)
  (CallFunction|SpawnPickups)
  (Utilities|FlowControl|Delay 1.0)
  (bind _asbp_game_state (Utilities|Casting|CastToBP_GameState (Game|GetGameState)))
  (Default|SERVERSetWaveCount _asbp_game_state (Variables|Default|GetcurrentWave) (Variables|Default|GetmaxWaves)))

(fn ConstructionScript)