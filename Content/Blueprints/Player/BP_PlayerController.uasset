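; Player controller that sets up local input and relays owner-side UI updates to BP_PlayerHUD.
; On local BeginPlay it adds the default Enhanced Input context, switches to game-only input, asks the game instance to hide the loading screen, then starts name and ping updates.
; OWNER events forward score, player name from the game instance, and attack UI show/hide to the HUD, while ping refreshes itself every second.
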(event Custom|OWNER_updateHUDName
  (bind _asbp_game_instance (Utilities|Casting|CastToBP_GameInstance (Game|GetGameInstance)))
  (bind _asbp_player_hud (Utilities|Casting|CastToBP_PlayerHUD (HUD|GetHUD)))
  (Default|OWNERUpdateHUDName _asbp_player_hud (Variables|/Game/Blueprints/BP_GameInstance.BP_GameInstance_C|GetplayerName _asbp_game_instance)))

(event Custom|OWNER_ShowAttackUI
  (bind _asbp_player_hud (Utilities|Casting|CastToBP_PlayerHUD (HUD|GetHUD)))
  (Default|OWNERShowAttackUI _asbp_player_hud))

(event Custom|OWNER_HideAttackUI
  (bind _asbp_player_hud (Utilities|Casting|CastToBP_PlayerHUD (HUD|GetHUD)))
  (Default|OWNERHideAttackUI _asbp_player_hud))

(event Custom|OWNER_updateHUDScore
  (bind _asbp_player_hud (Utilities|Casting|CastToBP_PlayerHUD (HUD|GetHUD)))
  (Default|OWNERUpdateHUDScore _asbp_player_hud))

(event Custom|OWNER_updateHUDPing
  (bind _asbp_player_hud (Utilities|Casting|CastToBP_PlayerHUD (HUD|GetHUD)))
  (Default|OWNERUpdateHUDPing _asbp_player_hud (Class|PlayerState|GetPinginMilliseconds (Variables|GetPlayerState)))
  (Utilities|FlowControl|Delay 1.0)
  (CallFunction|OWNERUpdateHUDPing))

(event EventBeginPlay
  (if (Pawn|IsLocalController)
    (Input|AddMappingContext (PlayerController|LocalPlayerSubsystems|GetEnhancedInputLocalPlayerSubsystem) "/Game/Input/IMC_Default.IMC_Default" 0 "(bIgnoreAllPressedKeysUntilRelease=True,bForceImmediately=False,bNotifyUserSettings=False)")
    (Variables|Default|SetbShowMouseCursor false)
    (Input|SetInputModeGameOnly self false)
    (bind _asbp_game_instance (Utilities|Casting|CastToBP_GameInstance (Game|GetGameInstance)))
    (Default|SERVERHideLoadingScreen _asbp_game_instance)
    (Utilities|FlowControl|Delay 0.5)
    (CallFunction|OWNERUpdateHUDName)
    (CallFunction|OWNERUpdateHUDPing)))

(fn ConstructionScript)