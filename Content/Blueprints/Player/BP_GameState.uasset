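; BP_GameState is the game state Blueprint that shares wave progress and match-over status with players.
; A server event relays current and max wave counts through a multicast, which stores them and passes them to the first player controller's wave count update.
; The IsMatchOver RepNotify tells that same BP_PlayerController to show the leaderboard when the match ends.
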(event Custom|SERVER_setWaveCount
  (params (currentWave :type Integer) (maxWaves :type Integer))
  (CallFunction|MULTISetWaveCount currentWave maxWaves))

(event Custom|MULTI_setWaveCount
  (params (currentWave :type Integer) (maxWaves :type Integer))
  (Variables|Default|SetcurrentWave currentWave)
  (Variables|Default|SetmaxWaves maxWaves)
  (bind _asbp_player_controller (Utilities|Casting|CastToBP_PlayerController (Game|GetPlayerController 0)))
  (Default|OWNERUpdateWaveCount _asbp_player_controller (Variables|Default|GetcurrentWave) (Variables|Default|GetmaxWaves)))

(fn ConstructionScript)

(fn OnRepIsMatchOver
  (if (Variables|Default|GetIsMatchOver)
    (bind _asbp_player_controller (Utilities|Casting|CastToBP_PlayerController (Game|GetPlayerController 0)))
    (Default|OWNERShowLeaderboard _asbp_player_controller)))