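; Player controller for the lobby that hands input to the lobby UI.
; On BeginPlay, the local controller casts its HUD to BP_LobbyHUD, sets UI-only input focused on that HUD's LobbyUI widget and shows the mouse cursor.
; On EndPlay, it removes that widget from its parent if still valid.
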(event EventBeginPlay
  (if (Pawn|IsLocalController)
    (bind _asbp_lobby_hud (Utilities|Casting|CastToBP_LobbyHUD (HUD|GetHUD)))
    (Input|SetInputModeUIOnly self (Variables|/Game/Blueprints/Lobby/BP_LobbyHUD.BP_LobbyHUD_C|GetlobbyUI _asbp_lobby_hud) "DoNotLock" false)
    (Variables|Default|SetbShowMouseCursor true)))

(event EventEndPlay
  (params (EndPlayReason :type EEndPlayReason%20Enum :default "Destroyed"))
  (bind _asbp_lobby_hud (Utilities|Casting|CastToBP_LobbyHUD (HUD|GetHUD)))
  (if (Utilities|IsValid (Variables|/Game/Blueprints/Lobby/BP_LobbyHUD.BP_LobbyHUD_C|GetlobbyUI _asbp_lobby_hud))
    (Widget|RemovefromParent (Variables|/Game/Blueprints/Lobby/BP_LobbyHUD.BP_LobbyHUD_C|GetlobbyUI _asbp_lobby_hud))))

(fn ConstructionScript)