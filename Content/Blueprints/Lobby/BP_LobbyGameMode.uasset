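; Lobby game mode that runs a ready-check countdown and then server-travels players to L_Main.
; TryStartCountdown requires every PlayerState to be ready, then writes the active flag and end time to the lobby GameState and starts a timer for the travel.
; CheckCountdownStillValid, run on logout, clears the timer and active flag if any player in the array is not ready.
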(event Custom|TryStartCountdown
  (if (CallFunction|AreAllPlayersReady)
    (bind _asbp_lobby_game_state (Utilities|Casting|CastToBP_LobbyGameState (Game|GetGameState)))
    (Variables|/Game/Blueprints/Lobby/BP_LobbyGameState.BP_LobbyGameState_C|SetisCountDownActive _asbp_lobby_game_state true)
    (bind _asbp_lobby_game_state_2 (Utilities|Casting|CastToBP_LobbyGameState (Game|GetGameState)))
    (Variables|/Game/Blueprints/Lobby/BP_LobbyGameState.BP_LobbyGameState_C|SetcountdownEndTime _asbp_lobby_game_state_2 (+ (Utilities|Time|GetGameTimeinSeconds) (Variables|Default|GetcountdownDuration)))
    (bind _returnvalue (Utilities|Time|SetTimerbyEvent (delegate Custom|StartMainLevel) (Variables|Default|GetcountdownDuration)))
    (Variables|Default|SetcountdownTimerHandle _returnvalue)))

(event Custom|StartMainLevel
  (Variables|/Game/Blueprints/Lobby/BP_LobbyGameState.BP_LobbyGameState_C|SetisCountDownActive (stale Custom|TryStartCountdown _asbp_lobby_game_state) false)
  (Development|ExecuteConsoleCommand "ServerTravel L_Main" 0))

(event EventOnLogout
  (params (ExitingController :type Controller%20Object%20Reference))
  (CallFunction|CheckCountdownStillValid))

(fn ConstructionScript)

(fn AreAllPlayersReady
  (bind _asbp_lobby_game_state (Utilities|Casting|CastToBP_LobbyGameState (Game|GetGameState)))
  (for _array_element (Variables|/Script/Engine.GameStateBase|GetPlayerArray _asbp_lobby_game_state)
    (bind _asbp_player_state (Utilities|Casting|CastToBP_PlayerState _array_element))
    (if (== (Variables|/Game/Blueprints/Player/BP_PlayerState.BP_PlayerState_C|GetisReady _asbp_player_state) false)
      (return false)))
  (return true))

(fn CheckCountdownStillValid
  (bind _asbp_lobby_game_state (Utilities|Casting|CastToBP_LobbyGameState (Game|GetGameState)))
  (if (Variables|/Game/Blueprints/Lobby/BP_LobbyGameState.BP_LobbyGameState_C|GetisCountDownActive _asbp_lobby_game_state)
    (if (not (CallFunction|AreAllPlayersReady))
      (Utilities|Time|ClearandInvalidateTimerbyHandle (Variables|Default|GetcountdownTimerHandle))
      (Variables|/Game/Blueprints/Lobby/BP_LobbyGameState.BP_LobbyGameState_C|SetisCountDownActive _asbp_lobby_game_state false))))