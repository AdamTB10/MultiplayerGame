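; BP_Attack is a projectile actor that makes players lose points when it hits them.
; Tick pushes it forward along local X and spins its mesh by fixed steps, not scaled by delta time.
; On Sphere1 overlap with a BP_Player, the authority has the player state play a hit sound and deduct points, doubled inside the centre area, then destroys the projectile.
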(event OnComponentBeginOverlap(Sphere1)
  (params (OverlappedComponent :type Primitive%20Component%20Object%20Reference) (OtherActor :type Actor%20Object%20Reference) (OtherComp :type Primitive%20Component%20Object%20Reference) (OtherBodyIndex :type Integer) (bFromSweep :type Boolean) (SweepResult :type Hit%20Result%20Structure%20%28by%20ref%29))
  (Networking|SwitchHasAuthority
    (:Authority
      (bind _asbp_player (Utilities|Casting|CastToBP_Player OtherActor))
      (bind _asbp_player_state (Utilities|Casting|CastToBP_PlayerState (Variables|/Script/Engine.Pawn|GetPlayerState _asbp_player)))
      (Default|OWNERPlayHitSound _asbp_player_state)
      (if (Variables|/Game/Blueprints/Player/BP_PlayerState.BP_PlayerState_C|GetisInCentreArea _asbp_player_state)
        (Variables|Default|SetpointsToLoose 4)
        (else
          (Variables|Default|SetpointsToLoose 2)))
      (Default|SERVERLoosePoints _asbp_player_state (Variables|Default|GetpointsToLoose))
      (Actor|DestroyActor))))

(event EventTick
  (params (DeltaSeconds :type Float%20%28single-precision%29))
  (Transformation|AddActorLocalOffset "50.000000,0.000000,0.000000" false false)
  (Transformation|AddWorldRotation (Variables|Default|GetStaticMesh) "25.000000,5.000000,10.000000" false false))

(fn ConstructionScript)