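; BP_HomingAttack is a homing projectile that makes the player it hits lose points.
; On BeginPlay the server ranks all players by distance, assumes the nearest is the thrower, and homes on the second nearest's TargetPoint.
; When its sphere overlaps a player, the server triggers a hit sound, deducts points (more if that player is in the centre area) and destroys the projectile.
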(event OnComponentBeginOverlap(Sphere1)
  (params (OverlappedComponent :type Primitive%20Component%20Object%20Reference) (OtherActor :type Actor%20Object%20Reference) (OtherComp :type Primitive%20Component%20Object%20Reference) (OtherBodyIndex :type Integer) (bFromSweep :type Boolean) (SweepResult :type Hit%20Result%20Structure%20%28by%20ref%29))
  (Networking|SwitchHasAuthority
    (:Authority
      (bind _asbp_player (Utilities|Casting|CastToBP_Player OtherActor))
      (bind _asbp_player_state (Utilities|Casting|CastToBP_PlayerState (Variables|/Script/Engine.Pawn|GetPlayerState _asbp_player)))
      (Default|OWNERPlayHitSound _asbp_player_state)
      (if (Variables|/Game/Blueprints/Player/BP_PlayerState.BP_PlayerState_C|GetisInCentreArea _asbp_player_state)
        (Variables|Default|SetpointsToLoose 6)
        (else
          (Variables|Default|SetpointsToLoose 3)))
      (Default|SERVERLoosePoints _asbp_player_state (Variables|Default|GetpointsToLoose))
      (Actor|DestroyActor))))

(event EventBeginPlay
  (bind _projectilemovement (Variables|Default|GetProjectileMovement))
  (Networking|SwitchHasAuthority
    (:Authority
      (bind _outactors (Actor|GetAllActorsOfClass "/Game/Blueprints/Player/BP_Player.BP_Player_C"))
      (bind _output_get (Variables|Default|SetallPlayers _outactors))
      (for _array_element _output_get
        (if (< (Transformation|GetDistanceTo _array_element self) (Variables|Default|GetclosestDistance))
          (Variables|Default|SetsecondClosestDistance (Variables|Default|GetclosestDistance))
          (Variables|Default|SettargetPlayer (Variables|Default|GetthrowingPlayer))
          (Variables|Default|SetclosestDistance (Transformation|GetDistanceTo _array_element self))
          (Variables|Default|SetthrowingPlayer _array_element)
          (elif (< (Transformation|GetDistanceTo _array_element self) (Variables|Default|GetsecondClosestDistance))
            (Variables|Default|SetsecondClosestDistance (Transformation|GetDistanceTo _array_element self))
            (Variables|Default|SettargetPlayer _array_element))))
      (Variables|/Script/Engine.ProjectileMovementComponent|SetHomingTargetComponent _projectilemovement (Variables|/Game/Blueprints/Player/BP_Player.BP_Player_C|GettargetPoint (Variables|Default|GettargetPlayer)))
      (Variables|/Script/Engine.ProjectileMovementComponent|SetHomingAccelerationMagnitude _projectilemovement (Variables|Default|Getspeed)))))

(fn ConstructionScript)