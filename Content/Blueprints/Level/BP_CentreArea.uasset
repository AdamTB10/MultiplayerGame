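; BP_CentreArea is a level trigger volume that tracks which players are inside the centre area.
; Its Box's begin and end overlap events run only on the authority and cast the overlapping actor to BP_Player.
; They then set IsInCentreArea on that player's BP_PlayerState to true on entry and false on exit.
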(event OnComponentBeginOverlap(Box)
  (params (OverlappedComponent :type Primitive%20Component%20Object%20Reference) (OtherActor :type Actor%20Object%20Reference) (OtherComp :type Primitive%20Component%20Object%20Reference) (OtherBodyIndex :type Integer) (bFromSweep :type Boolean) (SweepResult :type Hit%20Result%20Structure%20%28by%20ref%29))
  (Networking|SwitchHasAuthority
    (:Authority
      (bind _asbp_player (Utilities|Casting|CastToBP_Player OtherActor))
      (bind _asbp_player_state (Utilities|Casting|CastToBP_PlayerState (Variables|/Script/Engine.Pawn|GetPlayerState _asbp_player)))
      (Variables|/Game/Blueprints/Player/BP_PlayerState.BP_PlayerState_C|SetisInCentreArea _asbp_player_state true))))

(event OnComponentEndOverlap(Box)
  (params (OverlappedComponent :type Primitive%20Component%20Object%20Reference) (OtherActor :type Actor%20Object%20Reference) (OtherComp :type Primitive%20Component%20Object%20Reference) (OtherBodyIndex :type Integer))
  (Networking|SwitchHasAuthority
    (:Authority
      (bind _asbp_player (Utilities|Casting|CastToBP_Player OtherActor))
      (bind _asbp_player_state (Utilities|Casting|CastToBP_PlayerState (Variables|/Script/Engine.Pawn|GetPlayerState _asbp_player)))
      (Variables|/Game/Blueprints/Player/BP_PlayerState.BP_PlayerState_C|SetisInCentreArea _asbp_player_state false))))

(fn ConstructionScript)