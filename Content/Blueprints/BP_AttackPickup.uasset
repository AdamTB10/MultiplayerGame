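; BP_AttackPickup is a pickup actor that enables attacking for the player who touches it.
; It spins by a fixed step each Tick, while a timeline started on BeginPlay drives incremental vertical offsets.
; Box overlap is handled only with authority: it casts to BP_Player, calls SERVEREnableCanPlayerAttack on that player's BP_PlayerState, then destroys the pickup.
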(event OnComponentBeginOverlap(Box)
  (params (OverlappedComponent :type Primitive%20Component%20Object%20Reference) (OtherActor :type Actor%20Object%20Reference) (OtherComp :type Primitive%20Component%20Object%20Reference) (OtherBodyIndex :type Integer) (bFromSweep :type Boolean) (SweepResult :type Hit%20Result%20Structure%20%28by%20ref%29))
  (Networking|SwitchHasAuthority
    (:Authority
      (bind _asbp_player (Utilities|Casting|CastToBP_Player OtherActor))
      (bind _asbp_player_state (Utilities|Casting|CastToBP_PlayerState (Variables|/Script/Engine.Pawn|GetPlayerState _asbp_player)))
      (Default|SERVEREnableCanPlayerAttack _asbp_player_state)
      (Actor|DestroyActor))))

(event EventBeginPlay
  (bind _movement (Timeline|T_Movement Play)
    (:Update
      (Transformation|AddActorLocalOffset (Math|Vector|MakeVector 0.0 0.0 (* _movement 5.0)) false false))))

(event EventTick
  (params (DeltaSeconds :type Float%20%28single-precision%29))
  (Class|Actor|AddActorWorldRotation "0.000000,2.000000,0.000000"))

(fn ConstructionScript)